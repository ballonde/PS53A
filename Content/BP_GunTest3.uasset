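; BP_GunTest3 is a test gun whose main shot fires a BP_BulletBack projectile.
; MainShoot spawns the bullet at the Arrow component's transform, passes it DamageMainShot, then consumes main ammo through UseBulletMain.
; SecondaryShoot is empty, and its UseBulletSecondary call is left unconnected, so secondary fire does nothing.
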(event EventMainShoot
  (bind _returnvalue (Game|SpawnActorfromClass "/Game/BP_BulletBack.BP_BulletBack_C" (Transformation|GetWorldTransform (Variables|Default|GetArrow)) "Undefined" 0 0))
  (Variables|/Game/BP_BulletParent.BP_BulletParent_C|SetDamageBullet _returnvalue (Variables|Default|GetDamageMainShot))
  (CallFunction|UseBulletMain (Variables|Default|GetNbUseBulletByMainShot)))

(event EventSecondaryShoot)

(fn ConstructionScript
  (|CallParentFunction))