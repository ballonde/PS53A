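; BP_GunTest2 is a gun Blueprint with two fire modes built around continuous-damage bullets, overriding little beyond its shoot events.
; MainShoot spawns a BP_BulletContinusDamage at the Arrow's transform, passes it the main shot damage, then spends main ammo.
; SecondaryShoot spawns a BP_BulletSlowAndMarkContinusDamage at the same Arrow without setting damage, then spends secondary ammo.
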(event EventMainShoot
  (bind _returnvalue (Game|SpawnActorfromClass "/Game/BP_BulletContinusDamage.BP_BulletContinusDamage_C" (Transformation|GetWorldTransform (Variables|Default|GetArrow)) "Undefined" 0 0))
  (Variables|/Game/BP_BulletParent.BP_BulletParent_C|SetDamageBullet _returnvalue (Variables|Default|GetDamageMainShot))
  (CallFunction|UseBulletMain (Variables|Default|GetNbUseBulletByMainShot)))

(event EventSecondaryShoot
  (Game|SpawnActorfromClass "/Game/BP_BulletSlowAndMarkContinusDamage.BP_BulletSlowAndMarkContinusDamage_C" (Transformation|GetWorldTransform (Variables|Default|GetArrow)) "Undefined" 0 0)
  (CallFunction|UseBulletSecondary (Variables|Default|GetNbUseBulletBySecondaryShot)))

(fn ConstructionScript
  (|CallParentFunction))