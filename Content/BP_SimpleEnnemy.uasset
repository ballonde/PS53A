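; BP_SimpleEnnemy is an AI-driven enemy that runs a behavior tree when play begins.
; On BeginPlay it starts TestSimplEnnemy on its AI controller and sets up the TestSimpleEnnemy blackboard with its Target1 and Target2 objects.
; It then initializes current HP and speed from their max and initial values, steps skipped if no AI controller possesses it.
; Overlap and Tick events are disabled, leaving behavior to the tree.
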(event EventBeginPlay
  (|CallParentFunction)
  (bind _asaicontroller (Utilities|Casting|CastToAIController (Pawn|GetController)))
  (AI|RunBehaviorTree _asaicontroller "/Game/TestSimplEnnemy.TestSimplEnnemy")
  (bind _blackboardcomponent (Class|AIController|UseBlackboard _asaicontroller "/Game/TestSimpleEnnemy.TestSimpleEnnemy"))
  (bind _output_get (Variables|Default|SetBlackboard%20Component _blackboardcomponent))
  (AI|Components|Blackboard|SetValueasObject _output_get (Utilities|Name|MakeLiteralName "Target1") (Variables|Default|GetTarget1))
  (AI|Components|Blackboard|SetValueasObject _output_get (Utilities|Name|MakeLiteralName "Target2") (Variables|Default|GetTarget2))
  (Variables|Default|SetHPEnnemyCurrent (Variables|Default|GetHPEnnemymax))
  (Variables|Default|SetSpeedEnnemyCurrent (Variables|Default|GetSpeedEnnemyInitial)))

(event Collision|EventActorBeginOverlap
  (params (OtherActor :type Actor%20Object%20Reference))
  (|CallParentFunction OtherActor) ; This node is disabled and will not be called.\nDrag off pins to build functionality.
)

(event EventTick
  (params (DeltaSeconds :type Float%20%28single-precision%29))
  (|CallParentFunction DeltaSeconds) ; This node is disabled and will not be called.\nDrag off pins to build functionality.
)

(fn ConstructionScript
  (|CallParentFunction))