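; Base gun Blueprint that manages firing rate, magazine ammo and reloading.
; Fonctionnement fires through a DoOnce gate that resets after the shot delay, or triggers a timed, separately gated reload when the magazine empties.
; The base Shot passes zero to UseBullet, so it consumes no ammo itself.
; Shots and reloads push current and maximum ammo to the HUD through BP_PlayerController.
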(event Custom|Shot
  (CallFunction|UseBullet))

(event Custom|Fonctionnement
  (if (and (Variables|Default|GetDelayShotFinish) (> (Variables|Settings|GetNbBulletChargerCurrent) 0))
    (Utilities|FlowControl|DoOnce false :!label _label
      (:Completed
        (CallFunction|Shot)
        (CallFunction|UpdateDisplayUi)
        (if (<= (Variables|Settings|GetNbBulletChargerCurrent) 0)
          (CallFunction|Reloading)
          (else
            (Utilities|FlowControl|Delay (Variables|Settings|GetDelayShot))
            (goto _label Reset)))))))

(event Custom|UseBullet
  (params (NbBulletUse :type Integer))
  (Variables|Settings|SetNbBulletChargerCurrent (- (Variables|Settings|GetNbBulletChargerCurrent) NbBulletUse)))

(event Custom|Reloading
  (Utilities|FlowControl|DoOnce false :!label _label
    (:Completed
      (Utilities|FlowControl|Delay (Variables|Settings|GetTimeReloading))
      (Variables|Settings|SetNbBulletChargerCurrent (Variables|Settings|GetNbBulletChargerMaxCapacity))
      (Utilities|FlowControl|Sequence
        (:then_0
          (Utilities|FlowControl|DoOnce false) ; enters at Reset
        )
        (:then_1
          (CallFunction|UpdateDisplayUi))
        (:then_2
          (goto _label Reset))))))

(event Custom|UpdateDisplayUi
  (bind _asbp_player_controller (Utilities|Casting|CastToBP_PlayerController (Game|GetPlayerController 0)))
  (Default|UpdateDisplayGunInterface _asbp_player_controller (Utilities|Text|ToText(Integer) (Variables|Settings|GetNbBulletChargerMaxCapacity)) (Utilities|Text|ToText(Integer) (Variables|Settings|GetNbBulletChargerCurrent))))

(fn ConstructionScript)