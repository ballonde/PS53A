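; BP_SimpleEnnemy is an AI enemy that runs a behavior tree, seeding its Blackboard with a first target and the player.
; PawnSensing spotting the player sets PlayerVisible, switches to run speed and starts a debug-drawn line-of-sight trace.
; A clear hit within DistanceSight repeats the check once through a DoOnce gate.
; A blocked or too-distant hit calls LostPlayer, restoring walk speed, clearing PlayerVisible and resetting the gate.
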(event OnSeePawn(PawnSensing)
  (params (Pawn :type Pawn%20Object%20Reference))
  (Utilities|Casting|CastToFirstPersonCharacter Pawn)
  (Utilities|Casting|CastToBP_PlayerController (Game|GetPlayerController 0))
  (AI|Components|Blackboard|SetValueasBool (Variables|Default|GetBlackboard%20Component) (Utilities|Name|MakeLiteralName "PlayerVisible") true)
  (Variables|/Script/Engine.CharacterMovementComponent|SetMaxWalkSpeed (Variables|Character|GetCharacterMovement) (Variables|Default|GetRunSpeedEnnemyCurrent))
  (Variables|Default|SetTestSeePlayer true)
  (CallFunction|CheckSigth))

(event Custom|LostPlayer
  (Utilities|Casting|CastToFirstPersonCharacter (Game|Player|GetPlayerPawn 0))
  (Variables|/Script/Engine.CharacterMovementComponent|SetMaxWalkSpeed (Variables|Character|GetCharacterMovement) (Variables|Default|GetWalkSpeedEnnemyCurrent))
  (AI|Components|Blackboard|SetValueasBool (Variables|Default|GetBlackboard%20Component) (Utilities|Name|MakeLiteralName "PlayerVisible") false)
  (Variables|Default|SetTestSeePlayer false)
  (Utilities|FlowControl|DoOnce false) ; enters at Reset
)

(event Custom|checkSigth
  (if (Variables|Default|GetTestSeePlayer)
    (bind _asfirst_person_character (Utilities|Casting|CastToFirstPersonCharacter (Game|Player|GetPlayerPawn 0)))
    (bind (_outhit _returnvalue) (Collision|LineTraceByChannel (Transformation|GetActorLocation self) (Transformation|GetActorLocation _asfirst_person_character) "TraceTypeQuery3" false 0 "ForDuration" true "(R=1.000000,G=0.000000,B=0.000000,A=1.000000)" "(R=0.000000,G=1.000000,B=0.000000,A=1.000000)" 2.0))
    (if _returnvalue
      (if (<= (.Distance (Collision|BreakHitResult _outhit)) (Variables|Default|GetDistanceSight))
        (Utilities|Casting|CastToFirstPersonCharacter (.HitActor (Collision|BreakHitResult _outhit))
          (:then
            (Utilities|FlowControl|DoOnce false
              (:Completed
                (CallFunction|CheckSigth))))
          (:CastFailed
            (Variables|Default|SetTestSeePlayer false :!label _label)
            (CallFunction|LostPlayer)))
        (else
          (goto _label))))))

(event EventBeginPlay
  (|CallParentFunction)
  (bind _asaicontroller (Utilities|Casting|CastToAIController (Pawn|GetController)))
  (AI|RunBehaviorTree _asaicontroller "/Game/TestSimplEnnemy.TestSimplEnnemy")
  (bind _blackboardcomponent (Class|AIController|UseBlackboard _asaicontroller "/Game/TestSimpleEnnemy.TestSimpleEnnemy"))
  (bind _output_get (Variables|Default|SetBlackboard%20Component _blackboardcomponent))
  (AI|Components|Blackboard|SetValueasObject _output_get (Utilities|Name|MakeLiteralName "TargetCurrent") (Utilities|Array|Get(acopy) (Variables|Default|GetListTarget)))
  (AI|Components|Blackboard|SetValueasObject (Variables|Default|GetBlackboard%20Component) (Utilities|Name|MakeLiteralName "Player") (Game|Player|GetPlayerPawn 0)))

(event Collision|EventActorBeginOverlap
  (params (OtherActor :type Actor%20Object%20Reference))
  (|CallParentFunction OtherActor) ; This node is disabled and will not be called.\nDrag off pins to build functionality.
)

(event EventTick
  (params (DeltaSeconds :type Float%20%28single-precision%29))
  (|CallParentFunction DeltaSeconds) ; This node is disabled and will not be called.\nDrag off pins to build functionality.
)

(fn ConstructionScript
  (|CallParentFunction))