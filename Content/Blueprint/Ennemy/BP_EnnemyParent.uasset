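; Base enemy Blueprint handling health, death rewards, loot and timed status effects.
; TakeDamage triggers Dead at zero HP, which raises the player controller's kill combo by difficulty type plus an airborne-player bonus, restarts a combo timer, then destroys the enemy.
; Before destruction, Loot may spawn an ammo box, with odds rising with player score.
; Immobilize, slow and mark conditions use delays to revert, while ContinusDamage is an empty stub.
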(event Custom|TakeDamage
  (params (DamageGet :type Float%20%28single-precision%29))
  (Variables|Default|SetHPEnnemyCurrent (- (Variables|Default|GetHPEnnemyCurrent) DamageGet))
  (if (<= (Variables|Default|GetHPEnnemyCurrent) 0.0)
    (CallFunction|Dead)))

(event Custom|Dead
  (bind _asbp_player_controller (Utilities|Casting|CastToBP_PlayerController (Game|GetPlayerController 0)))
  (if (Utilities|Enum|Equal(Enum) (Variables|Default|GetTypeEnnemi) "Facile")
    (Default|IncreaseComboKill _asbp_player_controller 3.0)
    (bind _asbp_player_controller_2 (Utilities|Casting|CastToBP_PlayerController (Game|GetPlayerController 0) :!label _label))
    (bind _asfirst_person_character (Utilities|Casting|CastToFirstPersonCharacter (Game|Player|GetPlayerPawn 0)))
    (if (AI|Components|NavMovement|IsFalling (Variables|/Script/Engine.Character|GetCharacterMovement _asfirst_person_character))
      (Default|IncreaseComboKill _asbp_player_controller_2 4.0)
      (else
        (Default|IncreaseComboKill _asbp_player_controller_2 2.0)))
    (Utilities|Time|ClearTimerbyFunctionName 0 "EndComboKillTimer")
    (Utilities|Time|SetTimerbyFunctionName _asfirst_person_character "EndComboKillTimer" 1e+01)
    (CallFunction|Loot)
    (Actor|DestroyActor)
    (elif (Utilities|Enum|Equal(Enum) (Variables|Default|GetTypeEnnemi) "Moyen")
      (Default|IncreaseComboKill _asbp_player_controller 5.0)
      (goto _label)
      (elif (Utilities|Enum|Equal(Enum) (Variables|Default|GetTypeEnnemi) "Difficile")
        (Default|IncreaseComboKill _asbp_player_controller 1e+01)
        (goto _label)))))

(event Custom|ContinusDamage)

(event Custom|CondSlow
  (params (DurationSlow :type Float%20%28single-precision%29))
  (Variables|/Script/Engine.CharacterMovementComponent|SetMaxWalkSpeed (Variables|Character|GetCharacterMovement) (/ (Variables|Default|GetWalkSpeedEnnemyCurrent) 2.0))
  (Utilities|FlowControl|Delay DurationSlow)
  (Variables|/Script/Engine.CharacterMovementComponent|SetMaxWalkSpeed (Variables|Character|GetCharacterMovement) (Variables|Default|GetWalkSpeedEnnemyInitial)))

(event Custom|CondImmo
  (params (DurationImmo :type Float%20%28single-precision%29))
  (Variables|/Script/Engine.CharacterMovementComponent|SetMaxWalkSpeed (Variables|Character|GetCharacterMovement) 0.0)
  (Utilities|FlowControl|Delay DurationImmo)
  (Variables|/Script/Engine.CharacterMovementComponent|SetMaxWalkSpeed (Variables|Character|GetCharacterMovement) (Variables|Default|GetWalkSpeedEnnemyInitial)))

(event Custom|Loot
  (bind _asbp_player_controller (Utilities|Casting|CastToBP_PlayerController (Game|GetPlayerController 0)))
  (if (<= (Math|Random|RandomInteger 100) (Math|Float|Truncate (+ (* 10 (/ (Variables|/Game/Blueprint/BP_PlayerController.BP_PlayerController_C|GetScore _asbp_player_controller) 1e+02)) 1e+01)))
    (Game|SpawnActorfromClass "/Game/Blueprint/BP_LootMunBoxMainBullet.BP_LootMunBoxMainBullet_C" (Transformation|GetActorTransform self) "Undefined" 0 0)))

(event Custom|CondMarked
  (params (DurationMark :type Float%20%28single-precision%29))
  (Variables|Default|SetIsMarked? true)
  (Utilities|FlowControl|Delay DurationMark)
  (Variables|Default|SetIsMarked? false))

(event EventBeginPlay
  (Variables|Default|SetHPEnnemyCurrent (Variables|Default|GetHPEnnemyMax))
  (bind _output_get (Variables|Default|SetWalkSpeedEnnemyCurrent (Variables|Default|GetWalkSpeedEnnemyInitial)))
  (Variables|/Script/Engine.CharacterMovementComponent|SetMaxWalkSpeed (Variables|Character|GetCharacterMovement) _output_get)
  (Variables|Default|SetRunSpeedEnnemyCurrent (Variables|Default|GetRunSpeedEnnemyInitial)))

(fn ConstructionScript)