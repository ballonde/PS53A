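; BP_LootMunBoxMainBullet is an ammo box pickup that grants random amounts of main and secondary bullets.
; Both amounts are rolled independently on BeginPlay.
; When a FirstPersonCharacter overlaps its Box, it passes both amounts to the first player's BP_PlayerController through its bullet update events, then destroys itself.
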(event OnComponentBeginOverlap(Box)
  (params (OverlappedComponent :type Primitive%20Component%20Object%20Reference) (OtherActor :type Actor%20Object%20Reference) (OtherComp :type Primitive%20Component%20Object%20Reference) (OtherBodyIndex :type Integer) (bFromSweep :type Boolean) (SweepResult :type Hit%20Result%20Structure%20%28by%20ref%29))
  (Utilities|Casting|CastToFirstPersonCharacter OtherActor)
  (bind _asbp_player_controller (Utilities|Casting|CastToBP_PlayerController (Game|GetPlayerController 0)))
  (Default|UpdateBulletSecondEvent _asbp_player_controller (Variables|Default|GetnbBulletSecond))
  (Default|UpdateBulletEvent _asbp_player_controller (Variables|Default|GetnbBulletMain))
  (Actor|DestroyActor))

(event EventBeginPlay
  (Variables|Default|SetnbBulletMain (Math|Random|RandomInteger 150))
  (Variables|Default|SetnbBulletSecond (Math|Random|RandomInteger 150)))

(event Collision|EventActorBeginOverlap
  (params (OtherActor :type Actor%20Object%20Reference)))

(event EventTick
  (params (DeltaSeconds :type Float%20%28single-precision%29)))

(fn ConstructionScript)