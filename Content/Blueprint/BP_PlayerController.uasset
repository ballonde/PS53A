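; Player controller that holds health, consumables and combo score, and creates the gun, score and player HUD widgets on BeginPlay.
; Using the selected consumable spends a counter, adds capped overdose and triggers its effect, with each first-time use of a consumable raising the cost multiplier.
; Wall, run, shoot and kill combos turn points into stepped, capped multipliers.
; EndCombo adds value times multiplier to score, while update events push state to the widgets.
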(event Custom|UpdateDisplayComboValue
  ;[1 1 1] Update Score Interface
  (Default|UpdateCombo (Variables|Default|GetUI_ScoreInterface) (Utilities|Text|ToText(Float) (Variables|ComboWall|GetValueComboWall) "HalfToEven") (Utilities|Text|ToText(Float) (Variables|ComboWall|GetMultiplierValueComboWall) "HalfToEven") (Utilities|Text|ToText(Float) (Variables|ComboRun|GetValueComboRun) "HalfToEven") (Utilities|Text|ToText(Float) (Variables|ComboRun|GetMultiplierValueComboRun) "HalfToEven") (Utilities|Text|ToText(Float) (Variables|ComboShoot|GetValueComboShoot) "HalfToEven") (Utilities|Text|ToText(Float) (Variables|ComboShoot|GetMultiplierValueComboShoot) "HalfToEven") (Utilities|Text|ToText(Float) (Variables|ComboKill|GetValueComboKill) "HalfToEven") (Utilities|Text|ToText(Float) (Variables|ComboKill|GetMultiplierValueComboKill) "HalfToEven")))

(event Custom|UpdateDisplayGunInterface
  (params (NbBulletMainShoot :type Text) (NbBulletSecondaryShoot :type Text))
  ;[1 1 1] Update Gun Interface
  (Default|UpdateDisplayBullet (Variables|Default|GetUI_GunInterface) 0 NbBulletMainShoot NbBulletSecondaryShoot))

(event Custom|ResetComboShoot
  ;[1 1 1] Combo:Reset-Increase-End
  (Variables|ComboShoot|SetValueComboShoot 0.0)
  (Variables|ComboShoot|SetMultiplierValueComboShoot 1.0)
  (CallFunction|UpdateDisplayScoreInterface))

(event Custom|IncreaseComboShot
  (params (ValuePoint :type Float%20%28single-precision%29))
  ;[1 1 1] Combo:Reset-Increase-End
  (bind _output_get (Variables|ComboShoot|SetValueComboShoot (+ ValuePoint (Variables|ComboShoot|GetValueComboShoot))))
  (if (> (* 5 (Math|Conversions|ToFloat(Integer) (Math|Conversions|ToInteger(Byte) (Class|KismetMathLibrary|FFloor64 (/ _output_get 1e+01))))) 5e+01)
    (Variables|ComboShoot|SetMultiplierValueComboShoot 1.5)
    (else
      (Variables|ComboShoot|SetMultiplierValueComboShoot (+ (/ (* 5 (Math|Conversions|ToFloat(Integer) (Math|Conversions|ToInteger(Byte) (Class|KismetMathLibrary|FFloor64 (/ _output_get 1e+01))))) 1e+02) 1.0))))
  (CallFunction|UpdateDisplayComboValue))

(event Custom|TakeDamage
  (params (DamageTaken :type Float%20%28single-precision%29))
  (Variables|Default|SetHpPlayerCurrent (- (Variables|Default|GetHpPlayerCurrent) DamageTaken))
  (CallFunction|UpdateLifeDisplay))

(event Custom|ResetPlayer
  (Variables|Default|SetHpPlayerCurrent (Variables|Default|GetHpPlayerMax))
  (CallFunction|UpdateLifeDisplay))

(event Custom|UpdateLifeDisplay
  (Default|UpdateLifeDisplay (Variables|Default|GetUI_PlayerInterface) (Utilities|Text|ToText(Float) (Variables|Default|GetHpPlayerCurrent) "HalfToEven")))

(event Custom|UpdateConsommableDisplay
  (Default|UpdateConsommableDisplay (Variables|Default|GetUI_PlayerInterface) (Utilities|Text|ToText(Float) (Variables|Default|GetCompteurConsommable) "HalfToEven")))

(event Custom|UseConsommable
  (bind _currentconsomable (Variables|Default|GetCurrentConsomable))
  (bind _costconsommable (Variables|/Game/Blueprint/PA_Conssomable.PA_Conssomable_C|GetCostConsommable _currentconsomable))
  (if (>= (Variables|Default|GetCompteurConsommable) (* (Variables|Default|GetMultiplicateurCostConso) _costconsommable))
    (Variables|Default|SetCompteurConsommable (- (Variables|Default|GetCompteurConsommable) (* (Variables|Default|GetMultiplicateurCostConso) _costconsommable)))
    (bind _output_get (Variables|Default|SetOverdoseValue (+ (Variables|/Game/Blueprint/PA_Conssomable.PA_Conssomable_C|GetCostConsommable _currentconsomable) (Variables|Default|GetOverdoseValue))))
    (if (> _output_get 1e+02)
      (Variables|Default|SetOverdoseValue 1e+02))
    (if (Variables|/Game/Blueprint/PA_Conssomable.PA_Conssomable_C|GetAlreadyUsed (Variables|Default|GetCurrentConsomable))
      _
      (else
        (Variables|/Game/Blueprint/PA_Conssomable.PA_Conssomable_C|SetAlreadyUsed (Variables|Default|GetCurrentConsomable) true)
        (CallFunction|UpdateNbConsommableUsed 1)
        (Variables|Default|SetMultiplicateurCostConso 1.0)
        (Variables|Default|SetMultiplicateurCostConso (+ (Variables|Default|GetMultiplicateurCostConso) (* (Variables|Default|GetnbConsommableCurrenttlyUsed) 0.1)))))
    (Default|EffectUseConsommable (Variables|Default|GetCurrentConsomable))
    (CallFunction|UpdateConsommableDisplay)))

(event Custom|SelectConsommable
  (params (CurrentConsomable :type PA%20Conssomable%20Object%20Reference))
  (Variables|Default|SetCurrentConsomable CurrentConsomable))

(event Custom|UpdateNbConsommableUsed
  (params (changement :type Integer))
  (Variables|Default|SetnbConsommableCurrenttlyUsed (+ (Variables|Default|GetnbConsommableCurrenttlyUsed) changement)))

(event Custom|ResetComboKill
  ;[1 1 1] Combo:Reset-Increase-End
  (Variables|ComboKill|SetValueComboKill 0.0)
  (Variables|ComboKill|SetMultiplierValueComboKill 1.0)
  (CallFunction|UpdateDisplayScoreInterface))

(event Custom|UpdateDisplayNameWeapon
  (params (NameGun :type Text))
  ;[1 1 1] Update Gun Interface
  (Default|UpdateNameWeapon (Variables|Default|GetUI_GunInterface) NameGun))

(event Custom|IncreaseComboKill
  (params (ValuePointKill :type Float%20%28single-precision%29))
  ;[1 1 1] Combo:Reset-Increase-End
  (bind _output_get (Variables|ComboKill|SetValueComboKill (+ (Variables|ComboKill|GetValueComboKill) ValuePointKill)))
  (if (> (* 5 (Math|Conversions|ToFloat(Integer) (Math|Conversions|ToInteger(Byte) (Class|KismetMathLibrary|FFloor64 (/ _output_get 1e+01))))) 8e+01)
    (Variables|ComboKill|SetMultiplierValueComboKill 1.5)
    (else
      (Variables|ComboKill|SetMultiplierValueComboKill (+ (/ (* 5 (Math|Conversions|ToFloat(Integer) (Math|Conversions|ToInteger(Byte) (Class|KismetMathLibrary|FFloor64 (/ _output_get 1e+01))))) 1e+02) 1.0))))
  (CallFunction|UpdateDisplayComboValue))

(event Custom|UpdateDisplayScoreValue
  ;[1 1 1] Update Score Interface
  (Default|UpdateScore (Variables|Default|GetUI_ScoreInterface) (Utilities|Text|ToText(Float) (Variables|Default|GetScore) "HalfToEven")))

(event Custom|UpdateDisplayScoreInterface
  (CallFunction|UpdateDisplayComboValue)
  (CallFunction|UpdateDisplayScoreValue))

(event Custom|EndCombo
  (params (ValueComboEnd :type Float%20%28single-precision%29) (ValueMultiplicateurComboEnd :type Float%20%28single-precision%29))
  (Variables|Default|SetScore (+ (Variables|Default|GetScore) (* ValueComboEnd ValueMultiplicateurComboEnd))))

(event Custom|ResetComboRun
  ;[1 1 1] Combo:Reset-Increase-End
  (Variables|ComboRun|SetMultiplierValueComboRun 1.0)
  (Variables|ComboRun|SetValueComboRun 0.0)
  (CallFunction|UpdateDisplayScoreInterface))

(event Custom|IncreaseComboWall
  (params (ValuePoint :type Float%20%28single-precision%29))
  ;[1 1 1] Combo:Reset-Increase-End
  (bind _output_get (Variables|ComboWall|SetValueComboWall (+ ValuePoint (Variables|ComboWall|GetValueComboWall))))
  (if (> (* 2 (Math|Conversions|ToFloat(Integer) (Math|Conversions|ToInteger(Byte) (Class|KismetMathLibrary|FFloor64 (/ _output_get 1e+01))))) 5e+01)
    (Variables|ComboWall|SetMultiplierValueComboWall 1.5)
    (else
      (Variables|ComboWall|SetMultiplierValueComboWall (+ (/ (* 2 (Math|Conversions|ToFloat(Integer) (Math|Conversions|ToInteger(Byte) (Class|KismetMathLibrary|FFloor64 (/ _output_get 1e+01))))) 1e+02) 1.0))))
  (CallFunction|UpdateDisplayComboValue))

(event Custom|ResetComboWall
  ;[1 1 1] Combo:Reset-Increase-End
  (Variables|ComboWall|SetMultiplierValueComboWall 1.0)
  (Variables|ComboWall|SetValueComboWall 0.0)
  (CallFunction|UpdateDisplayScoreInterface))

(event Custom|IncreaseComboRun
  (params (ValuePoint :type Float%20%28single-precision%29))
  ;[1 1 1] Combo:Reset-Increase-End
  (bind _output_get (Variables|ComboRun|SetValueComboRun (+ ValuePoint (Variables|ComboRun|GetValueComboRun))))
  (if (> (* 2 (Math|Conversions|ToFloat(Integer) (Math|Conversions|ToInteger(Byte) (Class|KismetMathLibrary|FFloor64 (/ _output_get 5.0))))) 8e+01)
    (Variables|ComboRun|SetMultiplierValueComboRun 1.8)
    (else
      (Variables|ComboRun|SetMultiplierValueComboRun (+ (/ (* 2 (Math|Conversions|ToFloat(Integer) (Math|Conversions|ToInteger(Byte) (Class|KismetMathLibrary|FFloor64 (/ _output_get 5.0))))) 1e+02) 1.0))))
  (CallFunction|UpdateDisplayComboValue))

(event EventBeginPlay
  (bind _returnvalue (UserInterface|CreateWidget "/Game/InterfaceWidget/WBP_GunEquippedDisplay.WBP_GunEquippedDisplay_C"))
  (bind _output_get (Variables|Default|SetUI_GunInterface _returnvalue))
  (UserInterface|Viewport|AddtoViewport _output_get 0)
  (bind _returnvalue_2 (UserInterface|CreateWidget "/Game/InterfaceWidget/WBP_Score.WBP_Score_C"))
  (bind _output_get_2 (Variables|Default|SetUI_ScoreInterface _returnvalue_2))
  (UserInterface|Viewport|AddtoViewport _output_get_2 0)
  (CallFunction|UpdateDisplayScoreInterface)
  (bind _returnvalue_3 (UserInterface|CreateWidget "/Game/InterfaceWidget/WBP_PlayerUI.WBP_PlayerUI_C"))
  (bind _output_get_3 (Variables|Default|SetUI_PlayerInterface _returnvalue_3))
  (UserInterface|Viewport|AddtoViewport _output_get_3 0)
  (Variables|Default|SetHpPlayerCurrent (Variables|Default|GetHpPlayerMax))
  (CallFunction|UpdateLifeDisplay)
  (CallFunction|UpdateConsommableDisplay)
  (CallFunction|SelectConsommable (Variables|Default|GetConsomableAgi))
  (Variables|/Game/Blueprint/PA_Conssomable.PA_Conssomable_C|SetAlreadyUsed (Variables|Default|GetConsomableAgi) false)
  (Variables|/Game/Blueprint/PA_Conssomable.PA_Conssomable_C|SetAlreadyUsed (Variables|Default|GetConsomableShield) false)
  (Variables|/Game/Blueprint/PA_Conssomable.PA_Conssomable_C|SetAlreadyUsed (Variables|Default|GetConsomableKill) false))

(event Input|ActionEvents|InputActionUseConsommable
  (params (Key :type Key%20Structure :default "None"))
  (:Pressed
    (CallFunction|UseConsommable)))

(event Input|KeyboardEvents|L
  (params (Key :type Key%20Structure :default "None"))
  (:Pressed
    (CallFunction|SelectConsommable (Variables|Default|GetConsomableKill))
    (CallFunction|UseConsommable)))

(event Input|KeyboardEvents|M
  (params (Key :type Key%20Structure :default "None"))
  (:Pressed
    (CallFunction|SelectConsommable (Variables|Default|GetConsomableShield))
    (CallFunction|UseConsommable)))

(fn ConstructionScript)