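; BP_GunTest1 is a test gun Blueprint that implements a main and a secondary fire mode.
; The main shot spawns a BP_BulletSimple at the Arrow component's transform, passes it the main-shot damage and consumes main ammo.
; The secondary shot spawns a BP_BulletImmo from the same transform and consumes secondary ammo, without setting damage on it.
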(event EventMainShoot
  (bind _returnvalue (Game|SpawnActorfromClass "/Game/Blueprint/Bullet/BP_BulletSimple.BP_BulletSimple_C" (Transformation|GetWorldTransform (Variables|Default|GetArrow)) "Undefined" 0 0))
  (Variables|/Game/Blueprint/Bullet/BP_BulletParent.BP_BulletParent_C|SetDamageBullet _returnvalue (Variables|Default|GetDamageMainShot))
  (CallFunction|UseBulletMain (Variables|Default|GetNbUseBulletByMainShot)))

(event EventSecondaryShoot
  (Game|SpawnActorfromClass "/Game/Blueprint/Bullet/BP_BulletImmo.BP_BulletImmo_C" (Transformation|GetWorldTransform (Variables|Default|GetArrow)) "Undefined" 0 0)
  (CallFunction|UseBulletSecondary (Variables|Default|GetNbUseBulletBySecondaryShot)))

(fn ConstructionScript
  (|CallParentFunction))