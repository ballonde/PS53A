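; Base gun Blueprint that handles main and secondary fire for weapons.
; Fonctionnement checks the selected mode's cooldown and player-controller ammo, calls MainShoot or SecondaryShoot, refreshes the gun UI, then starts that mode's delay.
; Main fire loops after its delay while auto-fire is authorized and selected.
; The base shoot events only call the controller's bullet-use functions with zero, with no projectile or hit logic.
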(event Custom|SecondaryShoot
  (bind _asbp_player_controller (Utilities|Casting|CastToBP_PlayerController (Game|GetPlayerController 0)))
  (Default|UseBulletSecondary _asbp_player_controller))

(event Custom|UpdateDisplayUi
  (bind _asbp_player_controller (Utilities|Casting|CastToBP_PlayerController (Game|GetPlayerController 0)))
  (Default|UpdateDisplayGunInterface _asbp_player_controller))

(event Custom|Fonctionnement
  (params (MainShoot :type Boolean) (AutoShoot :type Boolean))
  (Variables|Default|SetAutoShootSelected? AutoShoot)
  (bind _output_get (Variables|Default|SetMainShootSelected? MainShoot))
  (if _output_get :!label _label
    (bind _asbp_player_controller (Utilities|Casting|CastToBP_PlayerController (Game|GetPlayerController 0)))
    (if (and (Variables|SettingsMainShoot|GetDelayMainShootFinish) (>= (Variables|/Game/Blueprint/BP_PlayerController.BP_PlayerController_C|GetnbBulletMain _asbp_player_controller) (Variables|SettingsMainShoot|GetNbUseBulletByMainShot)))
      (if (Variables|Default|GetMainShootSelected?) :!label _label_2
        (CallFunction|MainShoot)
        (else
          (CallFunction|SecondaryShoot)))
      (CallFunction|UpdateDisplayUi)
      (if (Variables|Default|GetMainShootSelected?)
        (Variables|SettingsMainShoot|SetDelayMainShootFinish false)
        (Utilities|FlowControl|Delay (Variables|SettingsMainShoot|GetDelayMainShoot))
        (Variables|SettingsMainShoot|SetDelayMainShootFinish true)
        (if (Variables|Default|GetAutoShootAurized)
          (if (Variables|Default|GetAutoShootSelected?)
            (goto _label)))
        (else
          (Variables|SettingsSecondaryShoot|SetDelaySecondaryShootFinish false)
          (Utilities|FlowControl|Delay (Variables|SettingsSecondaryShoot|GetDelaySecondaryShoot))
          (Variables|SettingsSecondaryShoot|SetDelaySecondaryShootFinish true))))
    (else
      (bind _asbp_player_controller_2 (Utilities|Casting|CastToBP_PlayerController (Game|GetPlayerController 0)))
      (if (and (Variables|SettingsSecondaryShoot|GetDelaySecondaryShootFinish) (>= (Variables|/Game/Blueprint/BP_PlayerController.BP_PlayerController_C|GetnbBulletSecond _asbp_player_controller_2) (Variables|SettingsSecondaryShoot|GetNbUseBulletBySecondaryShot)))
        (goto _label_2)))))

(event Custom|MainShoot
  (bind _asbp_player_controller (Utilities|Casting|CastToBP_PlayerController (Game|GetPlayerController 0)))
  (Default|UseBulletMain _asbp_player_controller))

(fn ConstructionScript)