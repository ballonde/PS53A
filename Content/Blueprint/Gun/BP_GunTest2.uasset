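; Test gun Blueprint with two fire modes, each spawning a projectile at its Arrow component's transform.
; MainShoot spawns BP_BulletSimple and then sets its damage from DamageMainShot.
; SecondaryShoot spawns BP_BulletSlowAndMarkContinusDamage, named for slow and marked damage-over-time effects, without setting its damage.
; After spawning, each mode tells player 0's BP_PlayerController to consume that mode's bullet count, with no ammo check here.
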(event EventMainShoot
  (bind _returnvalue (Game|SpawnActorfromClass "/Game/Blueprint/Bullet/BP_BulletSimple.BP_BulletSimple_C" (Transformation|GetWorldTransform (Variables|Default|GetArrow)) "Undefined" 0 0))
  (Variables|/Game/Blueprint/Bullet/BP_BulletParent.BP_BulletParent_C|SetDamageBullet _returnvalue (Variables|Default|GetDamageMainShot))
  (bind _asbp_player_controller (Utilities|Casting|CastToBP_PlayerController (Game|GetPlayerController 0)))
  (Default|UseBulletMain _asbp_player_controller (Variables|Default|GetNbUseBulletByMainShot)))

(event EventSecondaryShoot
  (Game|SpawnActorfromClass "/Game/Blueprint/Bullet/BP_BulletSlowAndMarkContinusDamage.BP_BulletSlowAndMarkContinusDamage_C" (Transformation|GetWorldTransform (Variables|Default|GetArrow)) "Undefined" 0 0)
  (bind _asbp_player_controller (Utilities|Casting|CastToBP_PlayerController (Game|GetPlayerController 0)))
  (Default|UseBulletSecondary _asbp_player_controller (Variables|Default|GetNbUseBulletBySecondaryShot)))

(fn ConstructionScript
  (|CallParentFunction))