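; BP_GunTest3 is a gun Blueprint, apparently a test variant, whose main shot fires a BP_BulletBack projectile.
; MainShoot spawns the bullet at the Arrow component's transform, passes it the main-shot damage, then has BP_PlayerController deduct the ammo used.
; SecondaryShoot is empty, and its secondary ammo-use logic is left unconnected.
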(event EventMainShoot
  (bind _returnvalue (Game|SpawnActorfromClass "/Game/Blueprint/Bullet/BP_BulletBack.BP_BulletBack_C" (Transformation|GetWorldTransform (Variables|Default|GetArrow)) "Undefined" 0 0))
  (Variables|/Game/Blueprint/Bullet/BP_BulletParent.BP_BulletParent_C|SetDamageBullet _returnvalue (Variables|Default|GetDamageMainShot))
  (bind _asbp_player_controller (Utilities|Casting|CastToBP_PlayerController (Game|GetPlayerController 0)))
  (Default|UseBulletMain _asbp_player_controller (Variables|Default|GetNbUseBulletByMainShot)))

(event EventSecondaryShoot)

(fn ConstructionScript
  (|CallParentFunction))